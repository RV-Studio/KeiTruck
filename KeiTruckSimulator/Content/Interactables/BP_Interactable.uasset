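; BP_Interactable is a base interactable actor that shows a text prompt facing the player while it can be interacted with.
; The text starts hidden; IsInteractable turns the Rotator component toward the given player position and shows it, and IsNotInteractable hides it.
; LookAt builds that rotation from cross-product axes against world up.
; Interact is a placeholder that only prints a debug string.
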(event EventBeginPlay)

(event Collision|EventActorBeginOverlap
  (params (OtherActor :type Actor%20Object%20Reference)))

(event EventTick
  (params (DeltaSeconds :type Float%20%28single-precision%29)))

(fn ConstructionScript
  (Rendering|SetVisibility (Variables|Default|GetTextRender) false true))

(fn Interact
  (Development|PrintString "Is Interacting"))

(fn IsInteractable
  (params (Player%20Position :type Vector))
  (bind _rotator (Variables|Default|GetRotator))
  (bind _rotate (CallFunction|Lookat (Transformation|GetWorldLocation _rotator) Player%20Position))
  (Transformation|SetWorldRotation _rotator _rotate false false)
  (Rendering|SetVisibility (Variables|Default|GetTextRender) true true))

(fn IsNotInteractable
  (Rendering|SetVisibility (Variables|Default|GetTextRender) false false))

(fn Lookat
  (params (Eye :type Vector) (Center :type Vector))
  (bind _output_get (LocalVariables|SetX (Math|Vector|Normalize (- Center Eye))))
  (bind _output_get_2 (LocalVariables|SetY (Math|Vector|Normalize (Math|Vector|CrossProduct "0.000000,0.000000,1.000000" _output_get))))
  (bind _output_get_3 (LocalVariables|SetZ (Math|Vector|Normalize (Math|Vector|CrossProduct (LocalVariables|GetX) _output_get_2))))
  (return (Math|Rotator|MakeRotationfromAxes (LocalVariables|GetX) (LocalVariables|GetY) _output_get_3)))